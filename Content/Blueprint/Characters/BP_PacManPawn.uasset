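; Pac-Man player pawn that also drives round flow through PacManGameInstance.
; BeginPlay shows a "Ready..." countdown, then enables execution and movement; Tick re-enters this sequence whenever movement is disabled.
; Tick also clears the timed FR state and all-phantom-home flag after a delay.
; When every food item is eaten, it resets score and food count, announces the win and loads Level_2.
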(event EventBeginPlay
  (bind _returnvalue (Game|GetGameInstance))
  (bind _aspac_man_game_instance (Utilities|Casting|CastToPacManGameInstance _returnvalue))
  (Utilities|Set|Message _aspac_man_game_instance "Ready...")
  (Utilities|FlowControl|Delay 3.0)
  (bind _aspac_man_game_instance_2 (Utilities|Casting|CastToPacManGameInstance _returnvalue))
  (Utilities|Set|Exec _aspac_man_game_instance_2 true)
  (Utilities|Set|Message _aspac_man_game_instance_2 "Go !")
  (Utilities|Set|CanMove true)
  (Class|PacManPawn|ResetLastDirection))

(event Collision|EventActorBeginOverlap
  (params (OtherActor :type Actor%20Object%20Reference)))

(event EventTick
  (params (DeltaSeconds :type Float%20%28single-precision%29))
  (bind _returnvalue (Game|GetGameInstance))
  (Utilities|FlowControl|Sequence
    (:then_0
      (bind _returnvalue_2 (Class|GridPawn|CheckCanMove))
      (if (not _returnvalue_2)
        (bind _aspac_man_game_instance (Utilities|Casting|CastToPacManGameInstance _returnvalue))
        (Utilities|Set|Exec _aspac_man_game_instance false)
        (Utilities|FlowControl|Delay 1.0)
        (bind _aspac_man_game_instance_2 (Utilities|Casting|CastToPacManGameInstance _returnvalue))
        (Utilities|Set|Message _aspac_man_game_instance_2 "Ready...")
        (Utilities|FlowControl|Delay 3.0)
        (bind _aspac_man_game_instance_3 (Utilities|Casting|CastToPacManGameInstance _returnvalue))
        (Utilities|Set|Exec _aspac_man_game_instance_3 true)
        (Utilities|Set|Message _aspac_man_game_instance_3 "Go !")
        (Utilities|Set|CanMove true)
        (Class|PacManPawn|ResetLastDirection)))
    (:then_1
      (bind _aspac_man_game_instance_4 (Utilities|Casting|CastToPacManGameInstance _returnvalue))
      (bind _returnvalue_3 (Class|PacManGameInstance|CheckFR _aspac_man_game_instance_4))
      (if _returnvalue_3
        (Utilities|FlowControl|Delay 8.0)
        (Utilities|FlowControl|Sequence
          (:then_0
            (bind _aspac_man_game_instance_5 (Utilities|Casting|CastToPacManGameInstance _returnvalue))
            (Utilities|Set|FR _aspac_man_game_instance_5 false))
          (:then_1
            (bind _aspac_man_game_instance_6 (Utilities|Casting|CastToPacManGameInstance _returnvalue))
            (Utilities|Set|AllPhantomHome _aspac_man_game_instance_6 false)))))
    (:then_2
      (bind _aspac_man_game_instance_7 (Utilities|Casting|CastToPacManGameInstance _returnvalue))
      (bind _returnvalue_4 (Class|PacManGameInstance|CheckEatenFood _aspac_man_game_instance_7))
      (if (== _returnvalue_4 244)
        (Utilities|Casting|CastToPacManGameInstance _returnvalue)
        (bind _aspac_man_game_instance_8 (Utilities|Casting|CastToPacManGameInstance _returnvalue))
        (Utilities|Set|Score _aspac_man_game_instance_8)
        (Class|PacManGameInstance|ResetEatenFood _aspac_man_game_instance_8)
        (Utilities|Set|Message _aspac_man_game_instance_8 "You won ! Loading Level 2...")
        (Utilities|FlowControl|Delay 5.0)
        (Game|OpenLevel(byName) "Level_2")))))

(fn ConstructionScript)