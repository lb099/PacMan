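; Blueprint for Clyde, the orange Pac-Man ghost, handling its color change, apparently for frightened mode.
; Each Tick casts the game instance to PacManGameInstance and polls CheckFR.
; The Cube and Cylinder meshes get the blue material while CheckFR is true and the orange one otherwise, reassigned every frame rather than on state change.
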(event EventBeginPlay)

(event Collision|EventActorBeginOverlap
  (params (OtherActor :type Actor%20Object%20Reference)))

(event EventTick
  (params (DeltaSeconds :type Float%20%28single-precision%29))
  (bind _returnvalue (Game|GetGameInstance))
  (Utilities|FlowControl|Sequence
    (:then_0
      (bind _aspac_man_game_instance (Utilities|Casting|CastToPacManGameInstance _returnvalue))
      (bind _returnvalue_2 (Class|PacManGameInstance|CheckFR _aspac_man_game_instance))
      (if _returnvalue_2
        (Utilities|FlowControl|Sequence
          (:then_0
            (Rendering|Material|SetMaterial (Variables|Default|GetCube) 0 "/Game/Blueprint/Material/BP_BlueMaterial.BP_BlueMaterial"))
          (:then_1
            (Rendering|Material|SetMaterial (Variables|Default|GetCylinder) 0 "/Game/Blueprint/Material/BP_BlueMaterial.BP_BlueMaterial")))))
    (:then_1
      (bind _aspac_man_game_instance_2 (Utilities|Casting|CastToPacManGameInstance _returnvalue))
      (bind _returnvalue_3 (Class|PacManGameInstance|CheckFR _aspac_man_game_instance_2))
      (if (not _returnvalue_3)
        (Utilities|FlowControl|Sequence
          (:then_0
            (Rendering|Material|SetMaterial (Variables|Default|GetCube) 0 "/Game/Blueprint/Material/BP_OrangeMaterial.BP_OrangeMaterial"))
          (:then_1
            (Rendering|Material|SetMaterial (Variables|Default|GetCylinder) 0 "/Game/Blueprint/Material/BP_OrangeMaterial.BP_OrangeMaterial")))))))

(fn ConstructionScript)